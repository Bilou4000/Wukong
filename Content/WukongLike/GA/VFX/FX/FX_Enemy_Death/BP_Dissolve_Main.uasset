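; Enemy death effect actor that dissolves a skeletal mesh alongside a matching Niagara effect.
; A setup macro, run at construction and BeginPlay, pushes alpha, edge color and dissolve texture to both, creating dynamic material instances per slot.
; On BeginPlay a timeline then animates Alpha on the mesh materials and Niagara system together.
; An equivalent static mesh setup macro exists but is not executed.
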(event Custom|Update%20Data%20SK
  (Utilities|SKMeshSetupMacro (Variables|Default|GetSK_Niagara) (Variables|Default|GetSkeletalMesh)
    (:Completed
      (bind _newtrack_1 (Timeline|Timeline PlayFromStart)
        (:Update
          (Rendering|Material|SetScalarParameterValueonMaterials (Variables|Default|GetSkeletalMesh) "Alpha" _newtrack_1)
          (Niagara|SetNiagaraVariable(Float) (Variables|Default|GetSK_Niagara) "Alpha" _newtrack_1))))))

(event EventBeginPlay
  (CallFunction|UpdateDataSK))

(event Collision|EventActorBeginOverlap
  (params (OtherActor :type Actor%20Object%20Reference)))

(event EventTick
  (params (DeltaSeconds :type Float%20%28single-precision%29)))

(fn ConstructionScript
  (Utilities|SKMeshSetupMacro (Variables|Default|GetSK_Niagara) (Variables|Default|GetSkeletalMesh)))