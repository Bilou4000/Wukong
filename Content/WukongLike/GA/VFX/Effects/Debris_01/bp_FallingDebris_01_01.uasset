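; Falling debris effect actor that emits particle bursts with DirtDebris playback at random intervals.
; The construction script assigns the configurable Particle template to the particle component.
; On BeginPlay, if that template is valid, an endless loop waits a random delay, activates particles and DirtDebris, then deactivates particles after a random duration.
; DirtDebris stops one second after each burst, in parallel with the next wait.
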(event EventBeginPlay
  (bind _particlesystem (Variables|Default|GetParticleSystem))
  (Utilities|IsValid (Variables|Default|GetParticle)
    (:Is%20Valid
      (Components|Activation|SetAutoActivate _particlesystem false)
      (Components|Activation|Deactivate _particlesystem)
      (Utilities|FlowControl|Delay (Math|Random|RandomFloatinRange (Variables|Default|GetDelayMin) (Variables|Default|GetDelayMax)) :!label _label)
      (Components|Activation|Activate (Variables|Default|GetParticleSystem) false)
      (Audio|Components|Audio|Play (Variables|Default|GetDirt_Debris) 0.0)
      (Utilities|FlowControl|Delay (Math|Random|RandomFloatinRange (Variables|Default|GetDurationMin) (Variables|Default|GetDurationMax)))
      (Components|Activation|Deactivate (Variables|Default|GetParticleSystem))
      (Utilities|FlowControl|Sequence
        (:then_0
          (goto _label))
        (:then_1
          (Utilities|FlowControl|Delay 1.0)
          (Audio|Components|Audio|Stop (Variables|Default|GetDirt_Debris)))))))

(fn ConstructionScript
  (bind _particle (Variables|Default|GetParticle))
  (Utilities|IsValid _particle
    (:Is%20Valid
      (Effects|Components|ParticleSystem|SetTemplate (Variables|Default|GetParticleSystem) _particle))))