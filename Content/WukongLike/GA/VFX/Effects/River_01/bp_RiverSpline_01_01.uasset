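; River VFX Blueprint that lays a chain of spline mesh segments along an editable spline to form a river.
; The construction script divides the spline length by SplineMeshLength and adds one segment per whole interval, leaving any remainder uncovered.
; Each segment takes local positions and tangents from the spline, with tangents clamped to the segment length, and receives RiverMaterial.
; The event graph holds no active logic.
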(event EventBeginPlay)

(event Collision|EventActorBeginOverlap
  (params (OtherActor :type Actor%20Object%20Reference)))

(event EventTick
  (params (DeltaSeconds :type Float%20%28single-precision%29)))

(fn ConstructionScript
  (bind _splinemeshlength (Variables|Default|GetSplineMeshLength))
  (bind _spline (Variables|Default|GetSpline))
  (bind _spline_2 (Variables|Default|GetSpline))
  (for _index (range 0 (- (Math|Float|Truncate (/ (Spline|GetSplineLength (Variables|Default|GetSpline)) (Variables|Default|GetSplineMeshLength))) 1))
    (bind _returnvalue (AddComponent|AddSplineMeshComponent false))
    (bind _output_get (Variables|Default|SetSplineMesh _returnvalue))
    (SplineMesh|SetStartandEnd _output_get (Spline|GetLocationatDistanceAlongSpline _spline_2 (* _index (Variables|Default|GetSplineMeshLength)) "Local") (Math|Vector|ClampVectorSize (Spline|GetTangentatDistanceAlongSpline _spline_2 (* _index (Variables|Default|GetSplineMeshLength)) "Local") 0.0 _splinemeshlength) (Spline|GetLocationatDistanceAlongSpline _spline (* (+ _index 1) (Variables|Default|GetSplineMeshLength)) "Local") (Math|Vector|ClampVectorSize (Spline|GetTangentatDistanceAlongSpline _spline (* (+ _index 1) (Variables|Default|GetSplineMeshLength)) "Local") 0.0 _splinemeshlength) true :!class /Script/Engine.SplineMeshComponent)
    (Rendering|Material|SetMaterial (Variables|Default|GetSplineMesh) 0 (Variables|Default|GetRiverMaterial))))