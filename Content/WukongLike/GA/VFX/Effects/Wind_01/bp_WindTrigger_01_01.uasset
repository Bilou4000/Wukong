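; Trigger-volume actor that plays a configurable particle effect, apparently wind VFX, when a Character enters its box.
; The construction script assigns the Particle template, and BeginPlay keeps the system deactivated until triggered.
; On overlap it activates the particles and disables box collision, re-enabling it after a short delay unless TriggerOnce is set.
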(event OnComponentBeginOverlap(Box)
  (params (OverlappedComponent :type Primitive%20Component%20Object%20Reference) (OtherActor :type Actor%20Object%20Reference) (OtherComp :type Primitive%20Component%20Object%20Reference) (OtherBodyIndex :type Integer) (bFromSweep :type Boolean) (SweepResult :type Hit%20Result%20Structure%20%28by%20ref%29))
  (Utilities|Casting|CastToCharacter OtherActor)
  (Components|Activation|Activate (Variables|Default|GetParticleSystem) false)
  (Collision|SetCollisionEnabled (Variables|Default|GetBox) "NoCollision")
  (if (not (Variables|Default|GetTriggerOnce?))
    (Utilities|FlowControl|Delay 4.0)
    (Collision|SetCollisionEnabled (Variables|Default|GetBox) "QueryOnly")))

(event EventBeginPlay
  (bind _particlesystem (Variables|Default|GetParticleSystem))
  (Utilities|IsValid (Variables|Default|GetParticle)
    (:Is%20Valid
      (Components|Activation|SetAutoActivate _particlesystem false)
      (Components|Activation|Deactivate _particlesystem))))

(event Collision|EventActorBeginOverlap
  (params (OtherActor :type Actor%20Object%20Reference)))

(event EventTick
  (params (DeltaSeconds :type Float%20%28single-precision%29)))

(fn ConstructionScript
  (bind _particle (Variables|Default|GetParticle))
  (Utilities|IsValid _particle
    (:Is%20Valid
      (Effects|Components|ParticleSystem|SetTemplate (Variables|Default|GetParticleSystem) _particle))))