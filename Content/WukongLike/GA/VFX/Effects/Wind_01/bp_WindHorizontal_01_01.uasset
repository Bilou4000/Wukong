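; Horizontal wind VFX actor that plays a particle effect at random intervals.
; The construction script applies the Particle variable as the ParticleSystem component's template.
; On BeginPlay it disables auto-activation and deactivates the component, then loops forever, waiting a random delay between DelayMin and DelayMax before each activation without reset.
; Without a valid Particle, neither the template assignment nor the loop runs.
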(event EventBeginPlay
  (bind _particlesystem (Variables|Default|GetParticleSystem))
  (Utilities|IsValid (Variables|Default|GetParticle)
    (:Is%20Valid
      (Components|Activation|SetAutoActivate _particlesystem false)
      (Components|Activation|Deactivate _particlesystem)
      (Utilities|FlowControl|Delay (Math|Random|RandomFloatinRange (Variables|Default|GetDelayMin) (Variables|Default|GetDelayMax)) :!label _label)
      (Components|Activation|Activate (Variables|Default|GetParticleSystem) false)
      (goto _label))))

(event Collision|EventActorBeginOverlap
  (params (OtherActor :type Actor%20Object%20Reference)))

(event EventTick
  (params (DeltaSeconds :type Float%20%28single-precision%29)))

(fn ConstructionScript
  (bind _particle (Variables|Default|GetParticle))
  (Utilities|IsValid _particle
    (:Is%20Valid
      (Effects|Components|ParticleSystem|SetTemplate (Variables|Default|GetParticleSystem) _particle))))