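; Base puzzle wheel that turns in quarter steps and can be reset to its initial state.
; RotateWheel triggers camera shake and rumble on the player pawn, then a timeline lerps the Wheel component 90 degrees in yaw from the actor's rotation.
; ResetWheel replaces a rotated wheel by spawning a fresh instance of its own class at the same location and destroying itself, rather than rotating back.
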(event EventRotateWheel
  ;[1 1 1] Wheel Rotation
  (Class|BPICamera|CameraShake(Message) (Game|Player|GetPlayerPawn 0) 0.1 "/Game/WukongLike/PROG/GameModes/Input/ControllerRumble/FF_Wheel1.FF_Wheel1" "/Game/WukongLike/PROG/Character/Camera/cameraShakeType/CS_Wheel.CS_Wheel_C")
  (Variables|Default|SetoldRotation (Transformation|GetActorRotation))
  (bind _newtrack_0 (Timeline|Rotate PlayFromStart)
    (:Update
      (Transformation|SetRelativeRotation (Variables|Default|GetWheel) (Math|Rotator|Lerp(Rotator) (Variables|Default|GetoldRotation) (Math|Rotator|CombineRotators (Variables|Default|GetoldRotation) "90.000000,0.000000,0.000000") _newtrack_0 true) false false))
    (:Finished
      (Variables|Default|SetoldRotation "0, 0, 0"))))

(event EventResetWheel
  ;[1 1 1] Reset Wheel if rotated
  (if (Utilities|Operators|NotEqual(!=) :A (Variables|/Script/Engine.SceneComponent|GetRelativeRotation (Variables|Default|GetWheel)))
    (Game|SpawnActorfromClass (Utilities|GetClass self) (Math|Transform|MakeTransform (Transformation|GetActorLocation) "0, 0, 0" "1.000000,1.000000,1.000000") "AlwaysSpawn" "MultiplyWithRoot" 0 0)
    (Actor|DestroyActor)))

(fn ConstructionScript)