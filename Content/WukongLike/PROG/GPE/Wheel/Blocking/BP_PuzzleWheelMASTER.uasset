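; Master Blueprint for a puzzle wheel that turns a quarter turn left or right and persists its state.
; RotateWheel plays sound, shake and rumble, suspends player movement and uses a timeline to rotate the wheel while pinning the player to an anchor.
; On finish it restores walking and saves the rotation count under its display name, replacing the whole Wheelstate map.
; BeginPlay reloads that count to set the wheel's rotation.
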(event EventRotateWheel
  (params (PlayerAnchor :type Scene%20Component%20Object%20Reference) (Player :type Actor%20Object%20Reference))
  ;[1 1 1] Wheel Rotation
  (Class|BPICamera|CameraShake(Message) (Game|Player|GetPlayerPawn 0) 0.1 "/Game/WukongLike/PROG/GameModes/Input/ControllerRumble/FF_Wheel1.FF_Wheel1" "/Game/WukongLike/PROG/Character/Camera/cameraShakeType/CS_Wheel.CS_Wheel_C")
  (Class|BPIPlayer|SetMovementModeWheel(Message) Player "MOVE_None")
  (Math|Integer|IncrementInt (Variables|Default|GetrotationCount)
    (:%20%20
      (Variables|Default|SetoldRotation (Transformation|GetActorRotation))
      (Audio|PlaySound2D "/Game/WukongLike/PROG/Sound/SFX/World_Sounds/Wheel_Turning_Short.Wheel_Turning_Short" 1.0 1.0 0.0 0 0)
      (bind _newtrack_0 (Timeline|Rotate PlayFromStart)
        (:Update
          (Transformation|SetRelativeRotation (Variables|Default|GetWheel) (Math|Rotator|Lerp(Rotator) (Variables|Default|GetoldRotation) (Math|Rotator|CombineRotators (Variables|Default|GetoldRotation) (Math|Rotator|MakeRotator 0.0 (Math|Float|SelectFloat -9e+01 9e+01 (Variables|Default|GetturnRight)) 0.0)) _newtrack_0 true) false false)
          (Utilities|IsValid Player
            (:Is%20Valid
              (Transformation|SetActorLocation Player (Transformation|GetWorldLocation PlayerAnchor) false false) ; Update player's location to anchor
            )))
        (:Finished
          (Variables|Default|SetoldRotation "0, 0, 0")
          (Class|BPIPlayer|SetMovementModeWheel(Message) Player "MOVE_Walking")
          (bind _save (Class|BPICamera|GetSaveRef(Message) (Game|Player|GetPlayerPawn 0)))
          (Variables|/Game/WukongLike/PROG/GameModes/Save/BP_Save.BP_Save_C|Setwheelstate _save (Utilities|Map|MakeMap (Utilities|GetDisplayName self) (Variables|Default|GetrotationCount)))
          (bind _name (Class|BPICamera|GetSaveName(Message) (Game|Player|GetPlayerPawn 0)))
          (SaveGame|SaveGametoSlot _save _name)
          (Development|PrintString (Utilities|String|ToString(Integer) (.Value (Utilities|Map|Find (Variables|/Game/WukongLike/PROG/GameModes/Save/BP_Save.BP_Save_C|Getwheelstate _save) (Utilities|GetDisplayName self))))))))))

(event EventBeginPlay
  (bind _turnright (Variables|Default|GetturnRight))
  ;[1 1 1] LoadSave
  (bind _name (Class|BPICamera|GetSaveName(Message) (Game|Player|GetPlayerPawn 0)))
  (bind _returnvalue (SaveGame|DoesSaveGameExist _name))
  (if _returnvalue
    (bind _returnvalue_2 (SaveGame|LoadGamefromSlot _name))
    (bind _asbp_save (Utilities|Casting|CastToBP_Save _returnvalue_2))
    (if (.ReturnValue (Utilities|Map|Find (Variables|/Game/WukongLike/PROG/GameModes/Save/BP_Save.BP_Save_C|Getwheelstate _asbp_save) (Utilities|GetDisplayName self)))
      _
      (else
        _))
    (bind _output_get (Variables|Default|SetrotationCount (.Value (Utilities|Map|Find (Variables|/Game/WukongLike/PROG/GameModes/Save/BP_Save.BP_Save_C|Getwheelstate _asbp_save) (Utilities|GetDisplayName self)))))
    (Transformation|SetRelativeRotation (Variables|Default|GetWheel) (Utilities|Select :Index _output_get :Option%200 "0, 0, 0" :Option%201 (Math|Rotator|SelectRotator "-90.000000,0.000000,0.000000" "90.000000,0.000000,0.000000" _turnright) :Option%202 (Math|Rotator|SelectRotator "-180.000000,0.000000,0.000000" "180.000000,0.000000,0.000000" _turnright)) false false)))

(fn ConstructionScript)