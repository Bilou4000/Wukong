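; BP_PuzzleWheelFirst is a puzzle wheel variant that closes a door behind the player.
; When a BPI_Player actor overlaps DoorCloseCollision, a timeline stretches DoorParent's Z scale up from zero.
; ResetWheel resets by replacement: if the wheel has rotated or the door has scale, it spawns a fresh instance at its location, without copying rotation, and destroys itself.
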(event OnComponentBeginOverlap(DoorCloseCollision)
  (params (OverlappedComponent :type Primitive%20Component%20Object%20Reference) (OtherActor :type Actor%20Object%20Reference) (OtherComp :type Primitive%20Component%20Object%20Reference) (OtherBodyIndex :type Integer) (bFromSweep :type Boolean) (SweepResult :type Hit%20Result%20Structure%20%28by%20ref%29))
  ;[1 1 1] Close Door
  (if (Utilities|DoesObjectImplementInterface OtherActor "/Game/WukongLike/PROG/Character/Player/BPI_Player.BPI_Player_C")
    (bind _newtrack_0 (Timeline|LerpDoor PlayFromStart)
      (:Update
        (Transformation|SetRelativeScale3D (Variables|Default|GetDoorParent) (Math|Vector|MakeVector 1.0 1.0 (Math|Float|Lerp 0.0 22.0 _newtrack_0)))))))

(event EventResetWheel
  ;[1 1 1] RestoreDoor
  (if (or (Utilities|Operators|NotEqual(!=) :A (Variables|/Script/Engine.SceneComponent|GetRelativeRotation (Variables|Default|GetWheel))) (> (.z (Transformation|GetWorldScale (Variables|Default|GetDoorParent))) 0.0))
    (Game|SpawnActorfromClass (Utilities|GetClass self) (Math|Transform|MakeTransform (Transformation|GetActorLocation) "0, 0, 0" "1.000000,1.000000,1.000000") "AlwaysSpawn" "MultiplyWithRoot" 0 0)
    (Actor|DestroyActor)))

(fn ConstructionScript
  (|CallParentFunction))