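; Player-operated lever that either reveals a chain of islands or rotates the mill of its parent actor, with a camera focus on the objective.
; MoveLever accumulates axis input to drive the rotation timeline and sounds, activating at a threshold.
; Islands appear with staggered delays and, if time-limited, hide from the end as the lever resets; the mill path anchors the player and destroys listed objects.
; BeginPlay restores lever state from BP_Save by display name, otherwise hiding its islands.
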(event Custom|RotateLever
  (bind _activevalue (Variables|Default|GetactiveValue))
  (bind _leverrotationseed (Variables|Default|GetleverRotationSeed))
  (bind _returnvalue (* _activevalue _leverrotationseed))
  ;[1 1 1] Set Lever Rotation
  (bind _rotation (Timeline|RotationIncrementation SetNewTime)
    (:Update
      (Variables|Default|SetleverTimelinePos _returnvalue)
      (Transformation|SetRelativeRotation (Variables|Default|Getlever) (Math|Rotator|MakeRotator 0.0 _rotation 2.7e+02) false false)
      ;[1 1 1] Play sound
      (if (and (< (Variables|Default|GetleverTimelinePos) 10.5) (> (Variables|Default|GetleverTimelinePos) 7.0))
        (Utilities|FlowControl|DoOnce false
          (:Completed
            (Audio|PlaySound2D "/Game/WukongLike/PROG/Sound/SFX/World_Sounds/Player_Lever_Short.Player_Lever_Short" 1.0 0.8 0.0 0 0))))
      (if (> (Variables|Default|GetleverTimelinePos) 18.0)
        (Utilities|FlowControl|DoOnce false
          (:Completed
            (Audio|PlaySound2D "/Game/WukongLike/PROG/Sound/SFX/World_Sounds/Player_Lever_Short.Player_Lever_Short" 1.0 1.0 0.0 0 0)))))))

(event Custom|ShowIslands
  ;[0.5521 0.2502 0.2502] When Active
  ;;[1 1 1] Show Islands
  (Utilities|FlowControl|Delay (Variables|Default|GetappearingFirstIslandDuration))
  (bind _arrayelement (Utilities|ForEachLoopwithDelay (Variables|Default|GetislandRefs) (Variables|Default|GetDelayEachApparitions))
    (:loopBody
      (Default|ShowIsland _arrayelement)
      (if (Variables|Default|GettimeLimitIsland)
        (Utilities|FlowControl|Delay (+ (Variables|Default|GetshowIslandDuration) (Variables|Default|GetappearingFirstIslandDuration) (* (Utilities|Array|Length (Variables|Default|GetislandRefs)) (Variables|Default|GetDelayEachApparitions))))
        (bind _output (Utilities|ForEachLoopwithDelayfromEnd (Variables|Default|GetislandRefs) 1.2)
          (:then_0
            (Default|HideIsland _output)
            (CallFunction|ResetLeverRot)))))))

(event Custom|StopResetLever
  ;[1 1 1] Reset Lever if not activate
  (bind _rotation (Timeline|Timeline Stop)
    (:Update
      (Transformation|SetRelativeRotation (Variables|Default|Getlever) (Math|Rotator|MakeRotator 0.0 (Math|Float|Lerp (.pitch (Variables|/Script/Engine.SceneComponent|GetRelativeRotation (Variables|Default|Getlever))) -4e+01 _rotation) 2.7e+02) false false))
    (:Finished
      (CallFunction|ResetLever))))

(event Custom|RotateMill
  ;[0.5521 0.2502 0.2502] When Active
  ;;[1 1 1] Rotate Mill
  (Utilities|FlowControl|DoOnce false
    (:Completed
      (Transformation|SetWorldLocation (Variables|Default|GetplayerAnchor) (Transformation|GetActorLocation (Variables|Default|GetplayerRef)) false false) ; Update anchor to player's position
      (Class|BPIPuzzleWheel|RotateWheel(Message) (Actor|GetParentActor) (Variables|Default|GetplayerAnchor) (Variables|Default|GetplayerRef))
      (for _array_element (Variables|PuzzleWheel|GetobjectsToDestroy)
        (Actor|DestroyActor _array_element)))))

(event Custom|ResetCameraFocus
  ;[1 1 1] Activate Lever
  (Utilities|FlowControl|DoOnce false) ; enters at Reset
)

(event Custom|ResetSound1
  ;[1 1 1] Play sound
  (Utilities|FlowControl|DoOnce false) ; enters at Reset
)

(event Custom|ResetSound2
  ;[1 1 1] Play sound
  (Utilities|FlowControl|DoOnce false) ; enters at Reset
)

(event EventMoveLever
  (params (AxisValue :type Float%20%28double-precision%29) (Player :type Actor%20Object%20Reference))
  ;[1 1 1] Activate Lever
  (CallFunction|StopResetLever)
  (Variables|Default|SetplayerRef Player)
  (CallFunction|RotateLever)
  (bind _output_get (Variables|Default|SetactiveValue (+ (Variables|Default|GetactiveValue) (/ AxisValue 8.0))))
  (if (>= (* _output_get (Variables|Default|GetleverRotationSeed)) (Variables|Default|GetmaxActiveValue))
    (Variables|Default|SetisActive true)
    (Variables|Default|SetactiveValue (Variables|Default|GetmaxActiveValue))
    (if (!= (Utilities|Array|Length (Variables|Default|GetislandRefs)) 0)
      (CallFunction|ShowIslands)
      (else
        (Variables|Camera|Setactivate%20Object (Actor|GetParentActor))
        (Variables|Camera|SetLook%20Time 5.0)))
    (Utilities|FlowControl|Delay 0.3)
    (Utilities|FlowControl|DoOnce false
      (:Completed
        (Class|BPICamera|ShowObjectif(Message) (Game|Player|GetPlayerPawn 0) (Variables|Camera|GetObjectif%20Pos) (Variables|Camera|Getactivate%20Object) (Variables|Camera|GetY%20Offset) (Variables|Camera|GetLook%20Time))
        (Utilities|FlowControl|Delay 2.0)
        (if (== (Utilities|Array|Length (Variables|Default|GetislandRefs)) 0)
          (CallFunction|RotateMill))))))

(event EventResetLeverRot
  ;[1 1 1] Reset Lever if not activate
  (bind _rotation (Timeline|Timeline PlayFromStart)
    (:Update
      (Transformation|SetRelativeRotation (Variables|Default|Getlever) (Math|Rotator|MakeRotator 0.0 (Math|Float|Lerp (.pitch (Variables|/Script/Engine.SceneComponent|GetRelativeRotation (Variables|Default|Getlever))) -4e+01 _rotation) 2.7e+02) false false))
    (:Finished
      (CallFunction|ResetLever))))

(event EventResetLever
  ;[1 1 1] Reset Lever if not activate
  (Variables|Default|SetactiveValue 0.0)
  (Variables|Default|SetisActive false)
  (CallFunction|ResetSound1)
  (CallFunction|ResetSound2)
  (CallFunction|ResetCameraFocus))

(event EventBeginPlay
  ;[1 1 1] LoadSave
  (bind _name (Class|BPICamera|GetSaveName(Message) (Game|Player|GetPlayerPawn 0)))
  (bind _returnvalue (SaveGame|DoesSaveGameExist _name))
  (if _returnvalue
    (bind _returnvalue_2 (SaveGame|LoadGamefromSlot _name))
    (bind _asbp_save (Utilities|Casting|CastToBP_Save _returnvalue_2))
    (Variables|Default|SetsaveRef _asbp_save)
    (if (or (.Value (Utilities|Map|Find (Variables|/Game/WukongLike/PROG/GameModes/Save/BP_Save.BP_Save_C|GetleverActive _asbp_save) (Utilities|GetDisplayName self))) (not (.ReturnValue (Utilities|Map|Find (Variables|/Game/WukongLike/PROG/GameModes/Save/BP_Save.BP_Save_C|GetleverActive _asbp_save) (Utilities|GetDisplayName self)))))
      (Transformation|SetRelativeRotation (Variables|Default|Getlever) "40.000000,270.000000,0.000000" false false)
      (Variables|Default|SetisActive true)
      (else
        (for _array_element (Variables|Default|GetislandRefs) :!label _label
          (Utilities|IsValid _array_element
            (:Is%20Valid
              (Default|HideIsland _array_element))))))
    (else
      (goto _label))))

(fn ConstructionScript)

(fn GetIsActive
  (return (Variables|Default|GetisActive)))

(fn IsTimeLimit
  (return (Variables|Default|GettimeLimitIsland)))