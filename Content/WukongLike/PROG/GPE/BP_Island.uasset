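; BP_Island is a gameplay island actor that other logic can show or hide through two events.
; ShowIsland enables the Island collision, plays a timeline that slides the child actor along relative X, and unhides the actor after a short delay.
; HideIsland hides the actor and disables collision immediately, without rewinding the timeline.
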(event Custom|ShowIsland
  (Utilities|FlowControl|Sequence
    (:then_0
      (Collision|SetCollisionEnabled (Variables|Default|GetIsland) "QueryAndPhysics")
      (bind _newtrack_0 (Timeline|Timeline Play)
        (:Update
          (Transformation|SetRelativeLocation (Variables|Default|GetChildActor) (Math|Vector|MakeVector (Math|Float|Lerp 0.0 1.5e+02 _newtrack_0) 0.0 0.0) false false))))
    (:then_1
      (Utilities|FlowControl|Delay 0.2)
      (Rendering|SetActorHiddenInGame false))))

(event Custom|HideIsland
  (Rendering|SetActorHiddenInGame true)
  (Collision|SetCollisionEnabled (Variables|Default|GetIsland) "NoCollision"))

(event EventBeginPlay)

(fn ConstructionScript)