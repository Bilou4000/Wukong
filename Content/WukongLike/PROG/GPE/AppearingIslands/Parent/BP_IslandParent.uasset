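; Parent Blueprint for appearing islands, which show or hide a configurable island mesh with collision.
; The construction script and BeginPlay apply the mesh and material to the Island component.
; ShowIsland enables collision at once, then after a short delay unhides the actor and plays a Timeline driving the material's Alpha parameter.
; HideIsland hides the actor and disables collision immediately before reversing that Timeline, so the reverse fade runs unseen.
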(event Custom|ShowIsland
  (Utilities|FlowControl|Sequence
    (:then_0
      (Collision|SetCollisionEnabled (Variables|Default|GetIsland) "QueryAndPhysics"))
    (:then_1
      (Utilities|FlowControl|Delay 0.2)
      (Rendering|SetActorHiddenInGame false)
      (bind _newtrack_0 (Timeline|Timeline PlayFromStart)
        (:Update
          (Rendering|Material|SetScalarParameterValueonMaterials (Variables|Default|GetIsland) "Alpha" _newtrack_0))))))

(event Custom|HideIsland
  (Rendering|SetActorHiddenInGame true)
  (Collision|SetCollisionEnabled (Variables|Default|GetIsland) "NoCollision")
  (bind _newtrack_0 (Timeline|Timeline ReverseFromEnd)
    (:Update
      (Rendering|Material|SetScalarParameterValueonMaterials (Variables|Default|GetIsland) "Alpha" _newtrack_0))))

(event EventBeginPlay
  (Components|StaticMesh|SetStaticMesh (Variables|Default|GetIsland) (Variables|Default|GetmeshIsland))
  (Rendering|Material|SetMaterial (Variables|Default|GetIsland) 0 (Variables|Default|GetislandMaterial)))

(fn ConstructionScript
  (bind _island (Variables|Default|GetIsland))
  (bind _meshisland (Variables|Default|GetmeshIsland))
  (Utilities|IsValid _meshisland
    (:Is%20Valid
      (Components|StaticMesh|SetStaticMesh _island _meshisland)
      (Rendering|Material|SetMaterial _island 0 (Variables|Default|GetislandMaterial)))))