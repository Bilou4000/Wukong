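; Tutorial trigger volume that shows a tutorial card on the player's HUD while the player is inside its box.
; On BeginPlay it caches the first player controller's HUD as HUD_Player.
; Box overlaps from actors implementing BPI_Player show the card given by WidgetToShow on entry and hide it on exit.
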(event OnComponentBeginOverlap(Box)
  (params (OverlappedComponent :type Primitive%20Component%20Object%20Reference) (OtherActor :type Actor%20Object%20Reference) (OtherComp :type Primitive%20Component%20Object%20Reference) (OtherBodyIndex :type Integer) (bFromSweep :type Boolean) (SweepResult :type Hit%20Result%20Structure%20%28by%20ref%29))
  (if (Utilities|DoesObjectImplementInterface OtherActor "/Game/WukongLike/PROG/Character/Player/BPI_Player.BPI_Player_C")
    (Default|ShowTutoCard (Variables|Default|GetplayerHudRef) (Variables|Default|GetwidgetToShow))))

(event OnComponentEndOverlap(Box)
  (params (OverlappedComponent :type Primitive%20Component%20Object%20Reference) (OtherActor :type Actor%20Object%20Reference) (OtherComp :type Primitive%20Component%20Object%20Reference) (OtherBodyIndex :type Integer))
  (if (Utilities|DoesObjectImplementInterface OtherActor "/Game/WukongLike/PROG/Character/Player/BPI_Player.BPI_Player_C")
    (Default|HideTutoCard (Variables|Default|GetplayerHudRef))))

(event EventBeginPlay
  (bind _ashud_player (Utilities|Casting|CastToHUD_Player (HUD|GetHUD (Game|GetPlayerController 0))))
  (Variables|Default|SetplayerHudRef _ashud_player))

(fn ConstructionScript)