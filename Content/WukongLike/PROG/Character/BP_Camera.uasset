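; BP_Camera is a camera actor that spawns the player character and follows it around the level.
; On BeginPlay it spawns BP_Player at its own transform and stores the reference.
; Each Tick it snaps its location to the player's without sweeping, leaving rotation untouched.
; Its IA_Move input handler only prints a debug string and does not drive movement.
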(event Input|EnhancedActionEvents|EnhancedInputActionIA_Move
  (params (ActionValue :type Float%20%28double-precision%29) (ElapsedSeconds :type Float%20%28double-precision%29) (TriggeredSeconds :type Float%20%28double-precision%29) (InputAction :type Input%20Action%20Object%20Reference :default "/Game/WukongLike/PROG/GameModes/Input/IA_Move.IA_Move"))
  (:Started
    (Development|PrintString "Hello")))

(event EventBeginPlay
  ;[1 1 1] Spawn Camera
  (bind _returnvalue (Game|SpawnActorfromClass "/Game/WukongLike/PROG/Character/BP_Player.BP_Player_C" (Transformation|GetActorTransform) "AlwaysSpawn" "MultiplyWithRoot" 0 0))
  (Variables|Default|SetPlayerRef _returnvalue))

(event EventTick
  (params (DeltaSeconds :type Float%20%28single-precision%29))
  (Utilities|IsValid (Variables|Default|GetPlayerRef)
    (:Is%20Valid
      (Transformation|SetActorLocation (Transformation|GetActorLocation (Variables|Default|GetPlayerRef)) false false))))

(fn ConstructionScript)