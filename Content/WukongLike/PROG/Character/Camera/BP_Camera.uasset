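; Side-view player camera actor that also owns the save game, restoring or creating it on BeginPlay and writing checkpoints with camera, player and lever state.
; Tick moves it via CalculateCamPos, using axis locks, position blending and a screen-width box trace against walls.
; Timelines blend spring arm offset and FOV, drive idle drift, and pan to objectives and back with player input disabled.
; It also plays camera shake with force feedback.
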(event Custom|StopAnim
  ;[1 1 1] ShowObject
  (bind _newtrack_0 (Timeline|Timeline Stop)
    (:Update
      (Variables|Default|SettargetPos (Math|Vector|Lerp(Vector) (Variables|Default|GettargetPos) (Transformation|GetActorLocation (Variables|Refs|GetplayerRef)) _newtrack_0)))
    (:Finished
      (Variables|Default|SetinTransition false)
      (CallFunction|CameraParameter (Variables|showObjectif|GetoldOffset) (Variables|/Script/Engine.CameraComponent|GetFieldOfView (Variables|Default|GetCamera)) (Variables|/Game/WukongLike/PROG/Character/Camera/BP_CameraDataAsset.BP_CameraDataAsset_C|GetcameraLag (Variables|Refs|GetdataAsset)))
      (if (or (Variables|showObjectif|GetoldBlockX) (Variables|showObjectif|GetoldBlockY))
        (CallFunction|CamFixPosition (Variables|showObjectif|GetoldBlockX) (Variables|showObjectif|GetoldBlockY) (Variables|Default|GettargetPos))
        (Variables|Default|SetdoesShowObjectif false)))))

(event Custom|CameraIdleStart
  (bind _dataasset (Variables|Refs|GetdataAsset))
  (bind _idlemovement (Variables|/Game/WukongLike/PROG/Character/Camera/BP_CameraDataAsset.BP_CameraDataAsset_C|GetidleMovement _dataasset))
  (bind (_x _y) (Math|Vector2D|BreakVector2D _idlemovement))
  ;[1 1 1] IdleMove
  (if (|checkVelocity)
    (bind (_direction _alphaleft _alphaup) (Timeline|Timeline_1 Play)
      (:Update
        (Transformation|SetRelativeLocation (Variables|Default|GetCamera) (Math|Vector|MakeVector 0.0 (Math|Float|Lerp _x 0.0 _alphaleft) (Math|Float|Lerp (/ _y 2.0) 0.0 _alphaup)) false false)))
    (else
      (Timeline|Timeline_1 Reverse))))

(event EventCameraShake
  (params (cameraShake :type Float%20%28double-precision%29) (rumbleCurve :type Force%20Feedback%20Effect%20Object%20Reference) (shakeCurve :type Camera%20Shake%20Base%20Class%20Reference))
  (bind _returnvalue (Game|GetPlayerController 0))
  ;[1 1 1] CameraShake
  (Game|Feedback|ClientPlayForceFeedback _returnvalue rumbleCurve "None" false false false)
  (Game|Feedback|ClientStartCameraShake _returnvalue shakeCurve cameraShake "World" "0, 0, 0"))

(event EventBeginPlay
  (bind _camera (Variables|Default|GetCamera))
  (bind _dataasset (Variables|Refs|GetdataAsset))
  (bind _fov (Variables|/Game/WukongLike/PROG/Character/Camera/BP_CameraDataAsset.BP_CameraDataAsset_C|GetFOV _dataasset))
  ;[1 0.315 0.4148] Start
  (bind _returnvalue (SaveGame|DoesSaveGameExist (Variables|save|GetsaveName)))
  (if _returnvalue
    (bind _returnvalue_2 (SaveGame|LoadGamefromSlot (Variables|save|GetsaveName)))
    (bind _asbp_save (Utilities|Casting|CastToBP_Save _returnvalue_2))
    (Variables|save|SetsaveRef _asbp_save)
    (Variables|Default|Setoffset (Variables|/Game/WukongLike/PROG/GameModes/Save/BP_Save.BP_Save_C|Getcamera_offset (Variables|save|GetsaveRef)))
    (Variables|Default|SetblockX (Variables|/Game/WukongLike/PROG/GameModes/Save/BP_Save.BP_Save_C|Getcamera_blockX (Variables|save|GetsaveRef)))
    (Variables|Default|SetblockY (Variables|/Game/WukongLike/PROG/GameModes/Save/BP_Save.BP_Save_C|Getcamera_blockY (Variables|save|GetsaveRef)))
    (Variables|Default|SettargetPos (Variables|/Game/WukongLike/PROG/GameModes/Save/BP_Save.BP_Save_C|Getcamera_targetPos (Variables|save|GetsaveRef)))
    (Camera|SetFieldOfView _camera (Math|Float|SelectFloat (Variables|/Script/Engine.CameraComponent|GetFieldOfView _camera) (Variables|/Game/WukongLike/PROG/GameModes/Save/BP_Save.BP_Save_C|Getcamera_FOV (Variables|save|GetsaveRef)) (< (Variables|/Game/WukongLike/PROG/GameModes/Save/BP_Save.BP_Save_C|Getcamera_FOV (Variables|save|GetsaveRef)) 1e+02)))
    (Variables|Default|SettargetFOV (Math|Float|SelectFloat (Variables|/Script/Engine.CameraComponent|GetFieldOfView _camera) (Variables|/Game/WukongLike/PROG/GameModes/Save/BP_Save.BP_Save_C|Getcamera_FOV (Variables|save|GetsaveRef)) (< (Variables|/Game/WukongLike/PROG/GameModes/Save/BP_Save.BP_Save_C|Getcamera_FOV (Variables|save|GetsaveRef)) 1e+02)))
    (Variables|/Script/Engine.SpringArmComponent|SetCameraLagSpeed (Variables|Default|GetSpringArm) (Variables|/Game/WukongLike/PROG/GameModes/Save/BP_Save.BP_Save_C|Getcamera_lag (Variables|save|GetsaveRef)))
    (else
      (bind _returnvalue_3 (SaveGame|CreateSaveGameObject "/Game/WukongLike/PROG/GameModes/Save/BP_Save.BP_Save_C"))
      (Variables|/Game/WukongLike/PROG/GameModes/Save/BP_Save.BP_Save_C|Setcamera_offset _returnvalue_3 "0, 0, 0")
      (Variables|/Game/WukongLike/PROG/GameModes/Save/BP_Save.BP_Save_C|SetplayerPos _returnvalue_3 "0, 0, 0")
      (SaveGame|SaveGametoSlot _returnvalue_3 (Variables|save|GetsaveName))
      (Variables|save|SetsaveRef _returnvalue_3)
      (Camera|SetFieldOfView (Variables|Default|GetCamera) _fov)
      (Variables|Default|SettargetFOV _fov)
      (CallFunction|ResetCamera 0.0)))
  (bind _outactors (Actor|GetAllActorsOfClass "/Game/WukongLike/PROG/Character/Player/BP_Player.BP_Player_C"))
  (bind _output_get (Variables|Refs|SetplayerRef (Utilities|Array|Get(acopy) _outactors)))
  (Class|BPIPlayer|SetSaveRef(Message) _output_get (Variables|save|GetsaveRef))
  (bind _aspc_player (Utilities|Casting|CastToPC_Player (Game|GetPlayerController 0)))
  (Default|SetPlayerRef _aspc_player (Variables|Refs|GetplayerRef))
  (CallFunction|CameraIdleStart)
  (CallFunction|SaveCheckpoint (Transformation|GetActorLocation)))

(event EventResetCamera
  (params (exitSmooth :type Float%20%28double-precision%29))
  ;[1 1 1] ResetCameraInfo
  (CallFunction|CameraParameter (Variables|/Game/WukongLike/PROG/Character/Camera/BP_CameraDataAsset.BP_CameraDataAsset_C|GetstartOffset (Variables|Refs|GetdataAsset)) (Variables|/Game/WukongLike/PROG/Character/Camera/BP_CameraDataAsset.BP_CameraDataAsset_C|GetFOV (Variables|Refs|GetdataAsset)) exitSmooth)
  (Variables|Default|SetcameraReset true))

(event EventTick
  (params (DeltaSeconds :type Float%20%28single-precision%29))
  (bind _returnvalue (Game|GetPlayerController 0))
  (bind (_startpos _endpos) (|BoxPos))
  ;[0.4169 1 0.5275] Tick
  (|IncrementLerp DeltaSeconds)
  (bind (_outhit _returnvalue_2) (Collision|BoxTraceByChannel _startpos _endpos (Math|Vector|MakeVector (* (Math|Vector|Distance(Vector) (.WorldLocation (Class|PlayerController|DeprojectScreenPositiontoWorld _returnvalue 0.0 5.4e+02)) (.WorldLocation (Class|PlayerController|DeprojectScreenPositiontoWorld _returnvalue 1.92e+03 5.4e+02))) 18.0) 5.0 2.5e+02) "0, 0, 0" "TraceTypeQuery3" true 0 "None"))
  (Transformation|SetActorLocation (|CalculateCamPos _outhit _returnvalue_2) false false))

(event EventCameraParameter
  (params (offset :type Vector :default "0, 0, 0") (newFOV :type Float%20%28double-precision%29) (newCameraLag :type Float%20%28double-precision%29))
  (bind _springarm (Variables|Default|GetSpringArm))
  ;[1 1 1] ChangeCamPosition
  ;;[0 0 0] FollowingCamera
  (Variables|Default|SettargetFOV newFOV)
  (Utilities|FlowControl|Sequence
    (:then_0
      (CallFunction|CamFixPosition false false "0, 0, 0")
      (Variables|/Script/Engine.SpringArmComponent|SetCameraLagSpeed (Variables|Default|GetSpringArm) newCameraLag)
      (Variables|Default|Setoffset offset)
      (Variables|Default|SetpositionLerp 1.0)
      (Variables|Default|SetinTransition true)
      (bind _newtrack_0 (Timeline|Lerp PlayFromStart)
        (:Update
          (Transformation|SetRelativeLocation (Variables|Default|GetSpringArm) (Math|Vector|Lerp(Vector) (Variables|/Script/Engine.SceneComponent|GetRelativeLocation _springarm) (Variables|Default|Getoffset) _newtrack_0) false false)
          (Camera|SetFieldOfView (Variables|Default|GetCamera) (Math|Float|Lerp (Variables|/Script/Engine.CameraComponent|GetFieldOfView (Variables|Default|GetCamera)) (Variables|Default|GettargetFOV) _newtrack_0)))
        (:Finished
          (Variables|Default|SetinTransition false)
          (if (Variables|Default|GetcameraReset)
            (Variables|/Script/Engine.SpringArmComponent|SetCameraLagSpeed _springarm 7.0)
            (Variables|Default|SetcameraReset false)))))
    (:then_1
      (if (Variables|Default|GetdoesShowObjectif)
        (CallFunction|StopAnim)))))

(event EventShowObjectif
  (params (objectifPos :type Vector :default "0, 0, 0") (objectifGO :type Actor%20Object%20Reference) (yOffset :type Float%20%28double-precision%29) (lookTime :type Float%20%28double-precision%29))
  (bind _offset (Variables|Default|Getoffset))
  ;[1 1 1] ShowObject
  (|canShow objectifPos objectifGO)
  (Variables|showObjectif|SetoldOffset (Variables|Default|Getoffset))
  (Variables|showObjectif|SetoldTarget (Variables|Default|GettargetPos))
  (Variables|showObjectif|SetoldBlockX (Variables|Default|GetblockX))
  (Variables|showObjectif|SetoldBlockY (Variables|Default|GetblockY))
  (Variables|showObjectif|SetoldCameraLag (Variables|/Game/WukongLike/PROG/Character/Camera/BP_CameraDataAsset.BP_CameraDataAsset_C|GetcameraLag (Variables|Refs|GetdataAsset)))
  (Variables|Default|SetdoesShowObjectif true)
  (CallFunction|CameraParameter (Math|Vector|MakeVector yOffset 0.0 0.0) (Variables|/Script/Engine.CameraComponent|GetFieldOfView (Variables|Default|GetCamera)) 3.0)
  (Class|BPIPlayer|DisableAllInputs(Message) (Variables|Refs|GetplayerRef) false)
  (Variables|Default|SetblockX true)
  (Variables|Default|SetblockY true)
  (Variables|Default|SetinTransition true)
  (Variables|Default|SettargetPos (+ (Transformation|GetActorLocation objectifGO) (Math|Vector|MakeVector (* (.y _offset) -1.0) (.x _offset) (.z _offset))))
  (bind _newtrack_0 (Timeline|lerpPos PlayFromStart)
    (:Update
      (Variables|Default|SettargetPos (Math|Vector|Lerp(Vector) (Variables|Default|GettargetPos) (Math|Vector|SelectVector (Transformation|GetActorLocation objectifGO) objectifPos (Utilities|Operators|EqualEqual :A objectifPos)) _newtrack_0)))
    (:Finished
      (Variables|Default|SetinTransition false)
      (Utilities|FlowControl|Delay lookTime)
      (Utilities|FlowControl|Sequence
        (:then_0
          (Variables|Default|SetinTransition true)
          (bind _newtrack_0_2 (Timeline|Timeline PlayFromStart)
            (:Update
              (Variables|Default|SettargetPos (Math|Vector|Lerp(Vector) (Variables|Default|GettargetPos) (Transformation|GetActorLocation (Variables|Refs|GetplayerRef)) _newtrack_0_2)))
            (:Finished
              (Variables|Default|SetinTransition false)
              (CallFunction|CameraParameter (Variables|showObjectif|GetoldOffset) (Variables|/Script/Engine.CameraComponent|GetFieldOfView (Variables|Default|GetCamera)) (Variables|/Game/WukongLike/PROG/Character/Camera/BP_CameraDataAsset.BP_CameraDataAsset_C|GetcameraLag (Variables|Refs|GetdataAsset)))
              (if (or (Variables|showObjectif|GetoldBlockX) (Variables|showObjectif|GetoldBlockY))
                (CallFunction|CamFixPosition (Variables|showObjectif|GetoldBlockX) (Variables|showObjectif|GetoldBlockY) (Variables|Default|GettargetPos))
                (Variables|Default|SetdoesShowObjectif false)))))
        (:then_1
          (Utilities|FlowControl|Delay 0.5)
          (Class|BPIPlayer|DisableAllInputs(Message) (Variables|Refs|GetplayerRef) true))))))

(event EventCamFixPosition
  (params (BlockX :type Boolean) (BlockY :type Boolean) (targetPos :type Vector :default "0, 0, 0"))
  ;[1 1 1] ChangeCamPosition
  ;;[0 0 0] Fixe Camera
  (Variables|Default|SetblockX BlockX)
  (Variables|Default|SetblockY BlockY)
  (Variables|Default|SettargetPos targetPos)
  (Variables|Default|SetpositionLerp 0.0))

(event EventSaveCheckpoint
  (params (CheckpointLoc :type Vector :default "0, 0, 0"))
  (bind _playerref (Variables|Refs|GetplayerRef))
  (bind _saveref (Variables|save|GetsaveRef))
  ;[1 1 1] SaveCheckpoint
  (Utilities|Array|Add (Variables|/Game/WukongLike/PROG/GameModes/Save/BP_Save.BP_Save_C|GetactivatedCheckPoint _saveref) CheckpointLoc)
  (Variables|/Game/WukongLike/PROG/GameModes/Save/BP_Save.BP_Save_C|SetplayerPos _saveref (Transformation|GetActorLocation (Variables|Refs|GetplayerRef)))
  (Variables|/Game/WukongLike/PROG/GameModes/Save/BP_Save.BP_Save_C|Setcamera_targetPos _saveref (Variables|Default|GettargetPos))
  (Variables|/Game/WukongLike/PROG/GameModes/Save/BP_Save.BP_Save_C|Setcamera_offset _saveref (Variables|Default|Getoffset))
  (Variables|/Game/WukongLike/PROG/GameModes/Save/BP_Save.BP_Save_C|Setcamera_blockX _saveref (Variables|Default|GetblockX))
  (Variables|/Game/WukongLike/PROG/GameModes/Save/BP_Save.BP_Save_C|Setcamera_blockY _saveref (Variables|Default|GetblockY))
  (Variables|/Game/WukongLike/PROG/GameModes/Save/BP_Save.BP_Save_C|Setcamera_lag _saveref (Variables|/Script/Engine.SpringArmComponent|GetCameraLagSpeed (Variables|Default|GetSpringArm)))
  (Variables|/Game/WukongLike/PROG/GameModes/Save/BP_Save.BP_Save_C|Setcamera_FOV _saveref (Variables|Default|GettargetFOV))
  (Variables|/Game/WukongLike/PROG/GameModes/Save/BP_Save.BP_Save_C|SetwindIndex _saveref (Variables|/Game/WukongLike/PROG/Character/Player/BP_Player.BP_Player_C|GetWind%20Index _playerref))
  (Variables|/Game/WukongLike/PROG/GameModes/Save/BP_Save.BP_Save_C|SetdoubleJumpEnable _saveref (Variables|/Game/WukongLike/PROG/Character/Player/BP_Player.BP_Player_C|GetdoubleJumpEnable _playerref))
  (Variables|/Game/WukongLike/PROG/GameModes/Save/BP_Save.BP_Save_C|SetdashEnable _saveref (Variables|/Game/WukongLike/PROG/Character/Player/BP_Player.BP_Player_C|GetdashEnable _playerref))
  (bind _outactors (Actor|GetAllActorswithInterface "/Game/WukongLike/PROG/GPE/BPI_Interractible.BPI_Interractible_C"))
  (for _array_element _outactors
    (bind _output (Class|BPIInterractible|IsTimeLimit(Message) _array_element))
    (bind _isactive (Class|BPIInterractible|GetIsActive(Message) _array_element))
    (Utilities|Map|Add (Variables|/Game/WukongLike/PROG/GameModes/Save/BP_Save.BP_Save_C|GetleverActive (Variables|save|GetsaveRef)) (Transformation|GetActorLocation _array_element) (select _output false _isactive)))
  (SaveGame|SaveGametoSlot (Variables|save|GetsaveRef) (Variables|save|GetsaveName)))

(fn ConstructionScript)

(fn GetCharacter
  (return (Variables|Refs|GetplayerRef)))

(fn GetSaveName
  (return (Variables|save|GetsaveName)))

(fn GetSaveRef
  (return (Variables|save|GetsaveRef)))