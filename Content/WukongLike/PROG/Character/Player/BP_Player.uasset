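; Side-scrolling player character with X-axis movement, jump, dash, pushback and lever interaction.
; An overlap detector flags interface-implementing objects unless falling; interacting locks movement and redirects the move axis to the lever.
; Dash and pushback launch the character, weaker in air, with dash recharging on the ground.
; Damage reduces life, then after an invincibility delay messages the causer to re-enable its damage.
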(event OnComponentBeginOverlap(Detection)
  (params (OverlappedComponent :type Primitive%20Component%20Object%20Reference) (OtherActor :type Actor%20Object%20Reference) (OtherComp :type Primitive%20Component%20Object%20Reference) (OtherBodyIndex :type Integer) (bFromSweep :type Boolean) (SweepResult :type Hit%20Result%20Structure%20%28by%20ref%29))
  ;[1 1 1] If the player overlap a interractible object (lever)
  (if (AI|Components|NavMovement|IsFalling (Variables|Character|GetCharacterMovement))
    (Variables|Default|SetcanInterract false)
    (else
      (Variables|Default|SetcanInterract (Utilities|DoesObjectImplementInterface OtherActor "/Game/WukongLike/PROG/GPE/BPI_Interractible.BPI_Interractible_C"))
      (Variables|Default|SetleverRef OtherActor))))

(event OnComponentEndOverlap(Detection)
  (params (OverlappedComponent :type Primitive%20Component%20Object%20Reference) (OtherActor :type Actor%20Object%20Reference) (OtherComp :type Primitive%20Component%20Object%20Reference) (OtherBodyIndex :type Integer))
  ;[1 1 1] If the player overlap a interractible object (lever)
  (Variables|Default|SetcanInterract false))

(event EventTick
  (params (DeltaSeconds :type Float%20%28single-precision%29))
  (if (AI|Components|NavMovement|IsMovingonGround (Variables|Character|GetCharacterMovement))
    (Variables|Default|SetcanDash true)))

(event Game|Damage|EventAnyDamage
  (params (Damage :type Float%20%28single-precision%29) (DamageType :type Damage%20Type%20Object%20Reference) (InstigatedBy :type Controller%20Object%20Reference) (DamageCauser :type Actor%20Object%20Reference))
  ;[1 1 1] Get Damage
  (Variables|Default|Setlife (- (Variables|Default|Getlife) Damage))
  (Utilities|FlowControl|Delay (Variables|Default|GetinvincibleTime))
  (Class|BPIEnemy|ResetApplyDamage(Message) DamageCauser))

(event EventDash
  (if (Variables|Default|GetcanDash)
    (Variables|Default|SetcanDash false)
    (if (not (AI|Components|NavMovement|IsMovingonGround (Variables|Character|GetCharacterMovement)))
      (Variables|Default|SetdashForce 5e+02)
      (else
        (Variables|Default|SetdashForce 2e+03)))
    (Character|LaunchCharacter (Math|Vector|MakeVector (* (Math|Float|SelectFloat 1.0 -1.0 (> (.x (Transformation|GetActorForwardVector)) 0.0)) (Variables|Default|GetdashForce)) 0.0 0.0) false false)))

(event EventMove
  (params (Axis :type Float%20%28double-precision%29))
  ;[1 1 1] Movements
  (Variables|Default|SetmoveAxis Axis)
  (if (not (Variables|Default|GetcanMove))
    (if (Variables|Default|GetisInterracting)
      ;[1 1 1] Move Lever if is interracting
      (Class|BPIInterractible|MoveLever(Message) (Variables|Default|GetleverRef) (Variables|Default|GetmoveAxis) self))
    (else
      (Pawn|Input|AddMovementInput "1.000000,0.000000,0.000000" (Variables|Default|GetmoveAxis) false))))

(event EventStartJump
  ;[1 1 1] Movements
  (Character|Jump))

(event EventEndJump
  ;[1 1 1] Movements
  (Character|StopJumping))

(event EventInterract
  ;[1 1 1] Set Interract
  (if (Variables|Default|GetcanInterract)
    (if (Variables|Default|GetisInterracting)
      (Variables|Default|SetisInterracting false)
      (CallFunction|SetCanMove true)
      (else
        (Variables|Default|SetisInterracting true)
        (CallFunction|SetCanMove false)))))

(event EventCancelInterract
  ;[1 1 1] Set Interract
  (Variables|Default|SetisInterracting false)
  (CallFunction|SetCanMove true))

(event EventSetCanMove
  (params (newCanMove :type Boolean))
  ;[1 1 1] Set can move
  (bind _output_get (Variables|Default|SetcanMove newCanMove))
  (Development|PrintString (Utilities|String|ToString(Boolean) _output_get)))

(event EventPushBack
  (params (direction :type Float%20%28double-precision%29))
  ;[1 1 1] Push Back
  (if (not (AI|Components|NavMovement|IsMovingonGround (Variables|Character|GetCharacterMovement)))
    (Variables|Default|SetpushbackForce 1e+02)
    (else
      (Variables|Default|SetpushbackForce 1.5e+03)))
  (Character|LaunchCharacter (Math|Vector|MakeVector (* direction (Variables|Default|GetpushbackForce)) 0.0 0.0) false false))

(fn ConstructionScript)