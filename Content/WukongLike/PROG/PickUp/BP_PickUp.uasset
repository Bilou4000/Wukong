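; BP_PickUp is an ability-unlock pickup that grants the player a power, identified by PowerUnlocked, on sphere overlap.
; It plays an idle sound on spawn, then on touch sends the upgrade through BPI_Player, swaps audio, plays the UnlockAbilities level sequence and hides itself.
; After a short delay it shows a double jump or dash tutorial card via HUD_Player, then destroys itself.
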(event OnComponentBeginOverlap(Sphere)
  (params (OverlappedComponent :type Primitive%20Component%20Object%20Reference) (OtherActor :type Actor%20Object%20Reference) (OtherComp :type Primitive%20Component%20Object%20Reference) (OtherBodyIndex :type Integer) (bFromSweep :type Boolean) (SweepResult :type Hit%20Result%20Structure%20%28by%20ref%29))
  ;[1 1 1] Get Pick Up
  (if (Utilities|DoesObjectImplementInterface OtherActor "/Game/WukongLike/PROG/Character/Player/BPI_Player.BPI_Player_C")
    (Utilities|FlowControl|Sequence
      (:then_0
        (Class|BPIPlayer|GetUpgrade(Message) OtherActor (Variables|Default|GetpowerUnlocked))
        (Audio|PlaySound2D "/Game/WukongLike/PROG/Sound/SFX/Pickup_Immortal_Food/ImmortalFood_PowerUp.ImmortalFood_PowerUp" 1.0 1.0 0.0 0 0)
        (Audio|Components|Audio|Stop (stale EventBeginPlay _returnvalue))
        (bind _outactor (Sequencer|Player|CreateLevelSequencePlayer "/Game/FX/FX_Unlock_Abilities/UnlockAbilities.UnlockAbilities"))
        (Sequencer|Player|Play (Variables|/Script/LevelSequence.LevelSequenceActor|GetSequencePlayer _outactor) :!class /Script/MovieScene.MovieSceneSequencePlayer)
        (Rendering|SetActorHiddenInGame true))
      (:then_1
        (Utilities|FlowControl|Delay 0.2)
        (bind _ashud_player (Utilities|Casting|CastToHUD_Player (HUD|GetHUD (Game|GetPlayerController 0))))
        (if (Utilities|Enum|Equal(Enum) (Variables|Default|GetpowerUnlocked) "NewEnumerator0")
          (Default|ShowTutoCard _ashud_player "/Game/WukongLike/PROG/UI/Tuto/W_TutoDoubleJump.W_TutoDoubleJump_C")
          (else
            (Default|ShowTutoCard _ashud_player "/Game/WukongLike/PROG/UI/Tuto/W_TutoDash.W_TutoDash_C")))
        (Actor|DestroyActor)))))

(event EventBeginPlay
  ;[1 1 1] Play sound on start
  (bind _returnvalue (Audio|SpawnSoundatLocation "/Game/WukongLike/PROG/Sound/SFX/Pickup_Immortal_Food/ImmortalFood_Idle.ImmortalFood_Idle" (Transformation|GetActorLocation) "0, 0, 0" 5e+01 1.0 0.0 (Variables|Default|GetAttenuation%20Settings) 0 false)))

(fn ConstructionScript)