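; PC_Player is the player controller that turns Enhanced Input actions into messages sent to the controlled player reference.
; On BeginPlay it adds the character mapping context and switches to game-only input.
; Move, jump, interact and dash forward to the player reference, with the last move value cached as the jump direction.
; Pause asks HUD_Player to open the pause menu, and an unused save-deletion snippet remains.
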(event Custom|SetPlayerRef
  (params (Player%20Ref :type Actor%20Object%20Reference))
  (Variables|Default|SetPlayer%20Ref Player%20Ref))

(event Input|EnhancedActionEvents|EnhancedInputActionIA_Move
  (params (ActionValue :type Float%20%28double-precision%29) (ElapsedSeconds :type Float%20%28double-precision%29) (TriggeredSeconds :type Float%20%28double-precision%29) (InputAction :type Input%20Action%20Object%20Reference :default "/Game/WukongLike/PROG/GameModes/Input/IA_Move.IA_Move"))
  (bind _player_ref (Variables|Default|GetPlayer%20Ref))
  (:Triggered
    (Utilities|IsValid _player_ref
      (:Is%20Valid
        (Class|BPIPlayer|Move(Message) _player_ref ActionValue)
        (Variables|Default|SetJump%20Direction ActionValue))))
  (:Completed
    (Variables|Default|SetJump%20Direction 0.0)))

(event Input|EnhancedActionEvents|EnhancedInputActionIA_Jump
  (params (ActionValue :type Boolean) (ElapsedSeconds :type Float%20%28double-precision%29) (TriggeredSeconds :type Float%20%28double-precision%29) (InputAction :type Input%20Action%20Object%20Reference :default "/Game/WukongLike/PROG/GameModes/Input/IA_Jump.IA_Jump"))
  (bind _player_ref (Variables|Default|GetPlayer%20Ref))
  (:Started
    (Class|BPIPlayer|StartJump(Message) _player_ref (Variables|Default|GetJump%20Direction)))
  (:Completed
    (Class|BPIPlayer|EndJump(Message) _player_ref)))

(event Input|EnhancedActionEvents|EnhancedInputActionIA_Interract
  (params (ActionValue :type Boolean) (ElapsedSeconds :type Float%20%28double-precision%29) (TriggeredSeconds :type Float%20%28double-precision%29) (InputAction :type Input%20Action%20Object%20Reference :default "/Game/WukongLike/PROG/GameModes/Input/IA_Interract.IA_Interract"))
  (:Started
    (Class|BPIPlayer|Interract(Message) (Variables|Default|GetPlayer%20Ref)))
  (:Completed
    (Class|BPIPlayer|CancelInterract(Message) (Variables|Default|GetPlayer%20Ref))))

(event Input|EnhancedActionEvents|EnhancedInputActionIA_Dash
  (params (ActionValue :type Boolean) (ElapsedSeconds :type Float%20%28double-precision%29) (TriggeredSeconds :type Float%20%28double-precision%29) (InputAction :type Input%20Action%20Object%20Reference :default "/Game/WukongLike/PROG/GameModes/Input/IA_Dash.IA_Dash"))
  (:Started
    (Class|BPIPlayer|Dash(Message) (Variables|Default|GetPlayer%20Ref))))

(event Input|EnhancedActionEvents|EnhancedInputActionIA_Pause
  (params (ActionValue :type Boolean) (ElapsedSeconds :type Float%20%28double-precision%29) (TriggeredSeconds :type Float%20%28double-precision%29) (InputAction :type Input%20Action%20Object%20Reference :default "/Game/WukongLike/PROG/GameModes/Input/IA_Pause.IA_Pause"))
  (:Started
    (bind _ashud_player (Utilities|Casting|CastToHUD_Player (HUD|GetHUD)))
    (Default|PauseGame _ashud_player "/Game/WukongLike/PROG/UI/W_PauseMenu.W_PauseMenu_C")))

(event Input|EnhancedActionEvents|EnhancedInputActionIA_ResetSave
  (params (ActionValue :type Boolean) (ElapsedSeconds :type Float%20%28double-precision%29) (TriggeredSeconds :type Float%20%28double-precision%29) (InputAction :type Input%20Action%20Object%20Reference :default "/Game/WukongLike/PROG/GameModes/Input/IA_ResetSave.IA_ResetSave")))

(event EventBeginPlay
  (Input|AddMappingContext (PlayerController|LocalPlayerSubsystems|GetEnhancedInputLocalPlayerSubsystem) "/Game/WukongLike/PROG/GameModes/Input/AMC_Character.AMC_Character" 0 "(bIgnoreAllPressedKeysUntilRelease=True,bForceImmediately=False)")
  (Input|SetInputModeGameOnly self false))

(fn ConstructionScript)